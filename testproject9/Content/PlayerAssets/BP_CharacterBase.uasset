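; Base character Blueprint that handles weapon spawning, montage-driven switching, and supplying the active weapon's idle and walk animations.
; Two seconds after BeginPlay it spawns BP_WeaponBase at its socket and hides Mesh; the attach and switch nodes are unconnected.
; Switching stores a pending weapon and plays a montage; WeaponSwitchHandsDownNotify commits the swap and toggles Mesh visibility.
; IA_Shoot currently triggers a switch with no weapon supplied.
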(event Custom|SwitchActiveWeaponTo
  (params (NewActiveWeapon :type BP%20Weapon%20Base%20Object%20Reference))
  (Variables|Default|SetPendingNextActiveWeapon NewActiveWeapon)
  (Animation|Montage|PlayMontage (Variables|Character|GetMesh) "/Game/Animations/ASM_WeaponSwitch.ASM_WeaponSwitch"))

(event Custom|WeaponInInventory
  (params (NewParam :type BP%20Weapon%20Base%20Object%20Reference))
  (Rendering|SetVisibility (Variables|Character|GetMesh) false true))

(event Custom|WeaponInHand
  (Rendering|SetVisibility (Variables|Character|GetMesh) true true))

(event Custom|AcquireNewWeapon
  (params (WeaponClass :type BP%20Weapon%20Base%20Class%20Reference))
  (bind _self self)
  (bind _returnvalue (Game|SpawnActorfromClass WeaponClass (Transformation|GetSocketTransform (Variables|Character|GetMesh) (.EquipSocketName (Utilities|GetClassDefaults WeaponClass)) "RTS_World") "Undefined" "MultiplyWithRoot" _self _self))
  (CallFunction|WeaponinInventory _returnvalue))

(event Input|EnhancedActionEvents|EnhancedInputActionIA_Shoot
  (params (ActionValue :type Boolean) (ElapsedSeconds :type Float%20%28double-precision%29) (TriggeredSeconds :type Float%20%28double-precision%29) (InputAction :type Input%20Action%20Object%20Reference :default "/Game/Input/Actions/IA_Shoot.IA_Shoot"))
  (CallFunction|SwitchActiveWeaponto))

(event EventBeginPlay
  (Utilities|FlowControl|Delay 2.0)
  (CallFunction|AcquireNewWeapon "/Game/Blueprints/Weapons/BP_WeaponBase.BP_WeaponBase_C"))

(event Collision|EventActorBeginOverlap
  (params (OtherActor :type Actor%20Object%20Reference)))

(event EventTick
  (params (DeltaSeconds :type Float%20%28single-precision%29)))

(fn ConstructionScript)

(fn GetActiveWeaponAnims
  (bind _currentactiveweapon (Variables|Default|GetCurrentActiveWeapon))
  (return (Variables|/Game/Blueprints/Weapons/BP_WeaponBase.BP_WeaponBase_C|GetIdleAnim _currentactiveweapon) (Variables|/Game/Blueprints/Weapons/BP_WeaponBase.BP_WeaponBase_C|GetWalkAnim _currentactiveweapon)))

(fn WeaponSwitchHandsDownNotify
  (Utilities|FlowControl|Sequence
    (:then_0
      (Utilities|IsValid (Variables|Default|GetCurrentActiveWeapon)
        (:Is%20Valid
          (CallFunction|WeaponinInventory (Variables|Default|GetCurrentActiveWeapon)))))
    (:then_1
      (Variables|Default|SetCurrentActiveWeapon (Variables|Default|GetPendingNextActiveWeapon))
      (CallFunction|WeaponinHand))))