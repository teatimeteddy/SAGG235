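; BP_RangedWeapon is a weapon Blueprint that adds clip-and-inventory ammo reloading to its parent class.
; CanReload requires reserve ammo, a non-full clip and a permitting weapon state, ignoring the parent's result, while CanAttack just defers to the parent.
; On reload completion it moves ammo and updates the UI.
; Only the move-all-remaining-reserve case works, as the nodes for filling the clip from a larger reserve are disconnected.
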(event Custom|MoveAmmoToFillClip
  (if (not (> (Variables|Default|GetAmmoInInventory) (- (Variables|Default|GetClipCapacity) (Variables|Default|GetAmmoInClip))))
    (Variables|Default|SetAmmoInClip (+ (Variables|Default|GetAmmoInInventory) (Variables|Default|GetAmmoInClip)))
    (Variables|Default|SetAmmoInInventory 0)))

(event EventBeginPlay
  (|CallParentFunction) ; This node is disabled and will not be called.\nDrag off pins to build functionality.
)

(event EventTick
  (params (DeltaSeconds :type Float%20%28single-precision%29))
  (|CallParentFunction DeltaSeconds) ; This node is disabled and will not be called.\nDrag off pins to build functionality.
)

(event EventReloadCompleteNotify
  (|CallParentFunction)
  (CallFunction|MoveAmmotoFillClip)
  (CallFunction|UpdateUI))

(event Collision|EventActorBeginOverlap
  (params (OtherActor :type Actor%20Object%20Reference))
  (|CallParentFunction OtherActor) ; This node is disabled and will not be called.\nDrag off pins to build functionality.
)

(fn ConstructionScript
  (|CallParentFunction))

(fn CanAttack
  (bind _result (|CallParentFunction))
  (return _result))

(fn CanReload
  (|CallParentFunction)
  (return (Math|Boolean|ANDBoolean (> (Variables|Default|GetAmmoInInventory) 0) (< (Variables|Default|GetAmmoInClip) (Variables|Default|GetClipCapacity)) (Utilities|Enum|NotEqual(Enum) (Variables|Default|GetWeaponState) "NewEnumerator2"))))