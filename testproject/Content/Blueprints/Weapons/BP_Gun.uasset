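; Hitscan gun weapon Blueprint that fires when its inherited attack-commit anim notify event runs.
; It line traces on the Camera channel from the owner's eye viewpoint along its facing at near-unlimited range, ignoring owner and gun.
; It then applies base damage to the hit actor and spawns a Niagara burst aligned to the impact normal, without checking whether the trace hit.
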(event EventBeginPlay
  (|CallParentFunction) ; This node is disabled and will not be called.\nDrag off pins to build functionality.
)

(event Collision|EventActorBeginOverlap
  (params (OtherActor :type Actor%20Object%20Reference))
  (|CallParentFunction OtherActor) ; This node is disabled and will not be called.\nDrag off pins to build functionality.
)

(event EventTick
  (params (DeltaSeconds :type Float%20%28single-precision%29))
  (|CallParentFunction DeltaSeconds) ; This node is disabled and will not be called.\nDrag off pins to build functionality.
)

(event EventCommitAttackAnimNotify
  (bind _returnvalue (Components|GetOwner))
  (bind (_outlocation _outrotation) (Actor|GetActorEyesViewPoint _returnvalue))
  (|CallParentFunction)
  (bind _outhit (Collision|LineTraceByChannel _outlocation (+ _outlocation (* (Math|Vector|GetForwardVector _outrotation) 1e+12)) "TraceTypeQuery2" false (Utilities|Array|MakeArray (Components|GetOwner) self) "None"))
  (Game|Damage|ApplyDamage (.HitActor (Collision|BreakHitResult _outhit)) (Variables|Default|GetBase%20Damage) 0 self "/Script/Engine.DamageType")
  (Niagara|SpawnSystematLocation "/Game/Pack_Simple_Particle_Burst/01_Niagara_Systems/NS_Simple_Burst_Level_3.NS_Simple_Burst_Level_3" (.Location (Collision|BreakHitResult _outhit)) (Math|Rotator|MakeRotfromX (.Normal (Collision|BreakHitResult _outhit)))))

(fn ConstructionScript
  (|CallParentFunction))